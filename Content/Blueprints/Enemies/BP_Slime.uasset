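; Slime enemy that chases the player once pawn sensing detects a pawn and deals contact damage to actors overlapping its capsule.
; Sensing sets a flag and issues an AI move toward the player.
; AnyDamage lowers clamped health, and at zero increments the player wizard's kill count and destroys the slime.
; Separate custom damage, death and destroy functions are uncalled here, and the custom death check is disconnected.
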(event `self.PawnSensing.OnSeePawn`
  (params (Pawn :type "Pawn Object Reference"))
  (set `self.IsSeeingPlayer?` true)
  (`self.FollowPlayer`))

(event `FollowPlayer`
  (if (`self.IsSeeingPlayer?`)
    (`|AIMoveTo` self (0.0 0.0 0.0) (`GameplayStatics.GetPlayerCharacter` 0) 150.0)))

(event `self.ReceiveAnyDamage`
  (params (Damage :type "Float (single-precision)") (DamageType :type "DamageType Object Reference") (InstigatedBy :type "Controller Object Reference") (DamageCauser :type "Actor Object Reference"))
  ; Enemy Health
  (bind _output_get (set `self.Health` (`KismetMathLibrary.FClamp` (- (`self.Health`) Damage) 0.0 100.0)))
  (if (== _output_get 0.0)
    (`|ExecutionSequence`
      (:`then_0`
        (bind _asbp_wizard (cast `/Game/Blueprints/Wizard/BP_Wizard` (`GameplayStatics.GetPlayerCharacter` 0)))
        (`/Engine/EditorBlueprintResources/StandardMacros.IncrementInt` (`/Game/Blueprints/Wizard/BP_Wizard.KillCount` _asbp_wizard)))
      (:`then_1`
        (`self.K2_DestroyActor`)))))

(event `self.CapsuleComponent.OnComponentBeginOverlap`
  (params (OverlappedComponent :type "PrimitiveComponent Object Reference") (OtherActor :type "Actor Object Reference") (OtherComp :type "PrimitiveComponent Object Reference") (OtherBodyIndex :type Integer) (bFromSweep :type Boolean) (SweepResult :type "HitResult Structure (by ref)"))
  ; Enemy Damage
  (`GameplayStatics.ApplyDamage` OtherActor 15.0))

(fn `ApplyDamageCustom`
  (params (DamageAmount :type "Float (double-precision)"))
  (if (not (`self.bDead`))
    (bind _output_get (set `self.Health` (- (`self.Health`) DamageAmount)))))

(fn `DestroySelf`
  (`self.K2_DestroyActor`))

(fn `Die`
  (set `self.bDead` true)
  (`PrimitiveComponent.SetCollisionEnabled` (`self.CapsuleComponent`) "NoCollision"))

(fn `UserConstructionScript`)